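; BP_HO_GameMode is a game mode that registers each player joining the server and gives them a random name.
; On PostLogin it adds the controller to ConPlayers and calls AssignRandomName, which renames them to "User-" plus a random five-digit number.
; After a two-second delay it prints a console message, tagged as a GameMode warning, announcing that the named player connected.
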(event EventPostLogin
  (params (NewPlayer :type Player%20Controller%20Object%20Reference))
  (Utilities|FlowControl|Sequence
    (:then_0
      (Utilities|Array|Add (Variables|Default|GetConPlayers) NewPlayer)
      (CallFunction|AssignRandomName NewPlayer))
    (:then_1
      (Utilities|FlowControl|Delay 2.0)
      (Class|Konsole|PrinttoConsole "GameMode" "Warning" (Utilities|String|ToString(Text) (Utilities|Text|FormatText "\"{NewPlayerName}\" connected to the server." (PlayerState|GetPlayerName (Variables|/Script/Engine.Controller|GetPlayerState NewPlayer))))))))

(fn ConstructionScript)

(fn AssignRandomName
  (params (Controller :type Controller%20Object%20Reference))
  (Class|GameModeBase|ChangeName Controller (Utilities|String|Append "User-" (Utilities|String|ToString(Integer) (Math|Random|RandomIntegerinRange 10000 99999))) false))