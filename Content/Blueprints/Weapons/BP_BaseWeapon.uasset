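; BP_BaseWeapon is a base hitscan gun, owned by its parent BP_HO_Character.
; PrimaryFire deprojects a point near screen center and passes that direction and the muzzle location to BeginFire.
; BeginFire runs a debug-drawn Camera-channel line trace, plays the hands montage through FireBullet, and applies point damage on hit.
; The construction script tints the mesh with GunColor; template projectile and sound logic remains unconnected.
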(event Custom|FireBullet
  (params (Result :type Hit%20Result%20Structure) (Direction :type Vector))
  (Animation|Montage|MontagePlay (Components|SkeletalMesh|GetAnimInstance (Variables|/HyperionOnline/Blueprints/BP_HO_Character.BP_HO_Character_C|GetHands (Variables|Default|GetCharacter))) (Variables|Default|GetMontage%20to%20Play) 1.0 "MontageLength" 0.0 true))

(event Custom|BeginFire
  (params (Direction :type Vector) (Origin :type Vector) (Controller :type Player%20Controller%20Object%20Reference))
  (bind _outhit (Collision|LineTraceByChannel Origin (+ Origin (* Direction (Variables|Info|GetGunRange))) "TraceTypeQuery2" false (Utilities|Array|MakeArray (Variables|Default|GetCharacter)) "ForDuration"))
  (Variables|Default|SetOut%20Hit _outhit)
  (Utilities|FlowControl|Sequence
    (:then_0
      (CallFunction|FireBullet :Direction Direction))
    (:then_1
      (if (.bblockinghit (Variables|Default|GetOut%20Hit))
        (Utilities|IsValid (.hitactor (Variables|Default|GetOut%20Hit))
          (:Is%20Valid
            (Game|Damage|ApplyPointDamage (.hitactor (Variables|Default|GetOut%20Hit)) (Variables|Status|GetGunDamage) (Math|Vector|GetUnitDirection(Vector) (.tracestart (Variables|Default|GetOut%20Hit)) (.traceend (Variables|Default|GetOut%20Hit))) (Variables|Default|GetOut%20Hit) (Game|GetPlayerController 0) self "/Script/Engine.DamageType")
            (Development|PrintString "Damaged")))
        (else
          (Development|PrintString "Not Bang"))))))

(event EventBeginPlay
  (bind _asbp_hyperion_character (Utilities|Casting|CastToBP_HO_Character (Actor|GetParentActor)))
  (bind _output_get (Variables|Default|SetCharacter _asbp_hyperion_character))
  (Actor|SetOwner _output_get))

(event EventPrimaryFire
  (params (bIsShooting :type Boolean))
  (bind _returnvalue (Game|GetPlayerController 0))
  (if bIsShooting
    (CallFunction|BeginFire (.WorldDirection (Class|GameplayStatics|DeprojectScreentoWorld _returnvalue (- (/ (Viewport|GetViewportSize) 2.0) "(X=0.000000,Y=-10.000000)"))) (Transformation|GetWorldLocation (Variables|Default|GetMuzzle)) _returnvalue)))

(fn ConstructionScript
  (Rendering|Material|SetVectorParameterValueonMaterials (Variables|Default|GetGunMesh) "BodyColor" (Math|Conversions|ToVector(LinearColor) (Variables|Default|GetGunColor))))