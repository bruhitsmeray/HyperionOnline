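; Multiplayer first-person player character with crouch, sprint, health and death, weapons, HUD, overhead name tags and a Discord connection.
; Movement input runs locally and through server events; optional smooth crouch animates capsule height and traces headroom before standing.
; Separate weapon child actors serve owner and other players, while OnRep fills name tags that overlap shows.
; Tick updates aim and checks death; BeginPlay also posts delayed connection messages to chat.
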(event OnComponentBeginOverlap(NameWidgetRadius)
  (params (OverlappedComponent :type Primitive%20Component%20Object%20Reference) (OtherActor :type Actor%20Object%20Reference) (OtherComp :type Primitive%20Component%20Object%20Reference) (OtherBodyIndex :type Integer) (bFromSweep :type Boolean) (SweepResult :type Hit%20Result%20Structure%20%28by%20ref%29))
  (Utilities|Casting|CastToBP_HO_Character OtherActor)
  (Rendering|SetVisibility (Variables|Default|GetNameWidget) true false))

(event OnComponentEndOverlap(NameWidgetRadius)
  (params (OverlappedComponent :type Primitive%20Component%20Object%20Reference) (OtherActor :type Actor%20Object%20Reference) (OtherComp :type Primitive%20Component%20Object%20Reference) (OtherBodyIndex :type Integer))
  (Utilities|Casting|CastToBP_HO_Character OtherActor)
  (Rendering|SetVisibility (Variables|Default|GetNameWidget) false false))

(event Custom|BeginCrouch
  ;[1 1 1] Custom Events
  (if (Variables|Default|GetbUseSmoothCrouch)
    (Variables|Default|SetbIsCrouching true)
    (Variables|/Script/Engine.CharacterMovementComponent|SetMaxWalkSpeed (Variables|Character|GetCharacterMovement) (Variables|Default|GetBaseCrouchSpeed))
    (bind _alpha (Timeline|Timeline_1 Play)
      (:Update
        (Components|Capsule|SetCapsuleHalfHeight (Variables|Default|GetCapsuleComponent) (Math|Float|Lerp 9e+01 45.0 _alpha) true)))
    (else
      (Character|Crouch))))

(event Custom|StopCrouch
  (bind _capsulecomponent (Variables|Default|GetCapsuleComponent))
  (bind _returnvalue (Transformation|GetWorldLocation _capsulecomponent))
  ;[1 1 1] Custom Events
  (if (Variables|Default|GetbUseSmoothCrouch)
    (bind _returnvalue_2 (Collision|CapsuleTraceByChannel (+ _returnvalue "0, 0,45.000000") (+ _returnvalue "0, 0,90.000000") 34.0 9e+01 "TraceTypeQuery1" true 0 "None"))
    (if (not _returnvalue_2)
      (Variables|Default|SetbIsCrouching false)
      (Variables|/Script/Engine.CharacterMovementComponent|SetMaxWalkSpeed (Variables|Character|GetCharacterMovement) (Variables|Default|GetBaseWalkSpeed))
      (bind _alpha (Timeline|Timeline_1 Reverse)
        (:Update
          (Components|Capsule|SetCapsuleHalfHeight (Variables|Default|GetCapsuleComponent) (Math|Float|Lerp 9e+01 45.0 _alpha) true))))
    (else
      (Character|UnCrouch))))

(event Custom|UpdateNameWidgetReference
  (bind _ashyperion_ui_nametag (Utilities|Casting|CastToHyperionUI_Nametag (UserInterface|GetUserWidgetObject (Variables|Default|GetNameWidget))))
  (Variables|/HyperionUI/Widgets/Others/HyperionUI_Nametag.HyperionUI_Nametag_C|SetCharacter _ashyperion_ui_nametag self))

(event Custom|UpdateNameOnServer
  (params (PlayerName :type String))
  (Variables|Info|SetPlayerName PlayerName))

(event Custom|IdleGunAnim
  ;[1 1 1] GunIdleAnim
  (if (and (Utilities|IsMoving) (not (Variables|Default|GetbIsCrouching)))
    (CallFunction|PlayIdleAnim)
    (else
      (CallFunction|StopIdleAnim))))

(event Custom|StopIdleAnim
  ;[1 1 1] GunIdleAnim
  (Rendering|SetVisibility (Variables|Default|GetHands) true false)
  (bind _returnvalue (Timeline|AnimGun Reverse)
    (:Update
      (Transformation|SetRelativeRotation (Variables|Default|GetWeapon) (Math|Rotator|Lerp(Rotator) "0, 0, 0" "0,-90.000000,10.000000" _returnvalue) false false))))

(event Custom|PlayIdleAnim
  ;[1 1 1] GunIdleAnim
  (Rendering|SetVisibility (Variables|Default|GetHands) false false)
  (bind _returnvalue (Timeline|AnimGun Play)
    (:Update
      (Transformation|SetRelativeRotation (Variables|Default|GetWeapon) (Math|Rotator|Lerp(Rotator) "0, 0, 0" "0,-90.000000,10.000000" _returnvalue) false false))))

(event Custom|KillEventOnServer
  (CallFunction|KillEvent))

(event Custom|UpdateHealth
  (Default|CallOnTakeDamage))

(event Custom|KillEvent
  (if (< (Variables|Default|GetLocalCurrentHealth) 1.0)
    (Utilities|FlowControl|Sequence
      (:then_0
        (Variables|Default|SetLocalCurrentHealth 0.0))
      (:then_1
        (Utilities|FlowControl|Delay 0.2)
        (Actor|DestroyActor)))))

(event Custom|StopCrouchOnServer
  (CallFunction|StopCrouch))

(event Custom|BeginCrouchOnServer
  (CallFunction|BeginCrouch))

(event EventTick
  (params (DeltaSeconds :type Float%20%28single-precision%29))
  (CallFunction|UpdateAimRotation)
  (CallFunction|UpdateHealth)
  (CallFunction|KillEvent)
  (CallFunction|KillEventonServer))

(event Game|Damage|EventAnyDamage
  (params (Damage :type Float%20%28single-precision%29) (DamageType :type Damage%20Type%20Object%20Reference) (InstigatedBy :type Controller%20Object%20Reference) (DamageCauser :type Actor%20Object%20Reference))
  (Variables|Default|SetLocalCurrentHealth (- (Variables|Default|GetLocalCurrentHealth) Damage)))

(event EventEndPlay
  (params (EndPlayReason :type EEndPlayReason%20Enum :default "Destroyed"))
  (CallFunction|DestroyDiscordConnection EndPlayReason))

(event EventBeginPlay
  (Utilities|FlowControl|Sequence
    (:then_0
      (Class|HOCharacter|ConnecttoDiscord 972531129770995732 false))
    (:then_1
      (Components|SkinnedMesh|HideBonebyName (Variables|Default|GetLegsMesh) "spine_01" "PBO_None")
      (Utilities|FlowControl|Delay 0.2)
      (CallFunction|ConfigureWeaponVisibility))
    (:then_2
      (CallFunction|AddHUD "/HyperionUI/HyperionUI_HUD.HyperionUI_HUD_C")
      (Utilities|FlowControl|Delay 2.0)
      (CallFunction|SendNametoServer))
    (:then_3
      (Utilities|FlowControl|Delay 1e+01)
      (bind _asbp_hyperion_game_mode (Utilities|Casting|CastToBP_HO_GameMode (Game|GetGameMode)))
      (for _array_element (Variables|/HyperionOnline/Blueprints/BP_HO_GameMode.BP_HO_GameMode_C|GetConPlayers _asbp_hyperion_game_mode)
        (bind _asbp_hyperion_controller (Utilities|Casting|CastToBP_HO_Controller (Game|GetPlayerController 0)))
        (Default|GetChatMessage _asbp_hyperion_controller "Server" (Utilities|Text|FormatText "{Player} connected to the server." (PlayerState|GetPlayerName (Variables|/Script/Engine.Controller|GetPlayerState _array_element))))))))

(event Input|ActionEvents|InputActionCrouch
  (params (Key :type Key%20Structure))
  (:Pressed
    (CallFunction|BeginCrouch)
    (CallFunction|BeginCrouchonServer))
  (:Released
    (CallFunction|StopCrouch)
    (CallFunction|StopCrouchonServer)))

(event Input|ActionEvents|InputActionSprint
  (params (Key :type Key%20Structure))
  (:Pressed
    (Class|HOCharacter|BeginSprint)
    (Class|HOCharacter|BeginSprintonServer))
  (:Released
    (Class|HOCharacter|StopSprint)
    (Class|HOCharacter|StopSprintonServer)))

(event Input|ActionEvents|InputActionShoot
  (params (Key :type Key%20Structure))
  (:Pressed
    (Class|BPICombat|PrimaryFire(Message) (Variables|/Script/Engine.ChildActorComponent|GetChildActor (Variables|Default|GetWeapon)) true)))

(event Input|ActionEvents|InputActionInterfaceMode
  (params (Key :type Key%20Structure))
  (:Pressed
    (Utilities|FlowControl|FlipFlop
      (:A
        (CallFunction|EnterInterfaceMode))
      (:B
        (CallFunction|DisableInterfaceMode)))))

(fn ConstructionScript)

(fn AddHUD
  (params (Class :type User%20Widget%20Class%20Reference))
  (bind _returnvalue (UserInterface|CreateWidget Class (Game|GetPlayerController 0)))
  (bind _output_get (Variables|Default|SetPlayerInterface _returnvalue))
  (Utilities|IsValid _output_get
    (:Is%20Valid
      (UserInterface|Viewport|AddtoViewport _output_get 0))
    (:Is%20Not%20Valid
      (Development|PrintString "User Widget Return Value Invalid." true true "(R=1.000000,G=0.000000,B=0.000000,A=1.000000)" 5.0))))

(fn EquipWeapon
  (params (bVisibility :type Boolean))
  (Rendering|SetVisibility (Variables|Default|GetHands) bVisibility false)
  (Rendering|SetVisibility (Variables|Default|GetWeapon) bVisibility false))

(fn UpdateAimRotation
  (Networking|SwitchHasAuthority
    (:Authority
      (Variables|Default|SetAimRotation (Pawn|GetControlRotation :!class /Script/Engine.Pawn)))))

(fn ConfigureWeaponVisibility
  (Utilities|FlowControl|Sequence
    (:then_0
      (bind _asbp_base_weapon (Utilities|Casting|CastToBP_BaseWeapon (Variables|/Script/Engine.ChildActorComponent|GetChildActor (Variables|Default|GetWeapon))))
      (Rendering|SetOnlyOwnerSee (Variables|/HyperionOnline/Blueprints/Weapons/BP_BaseWeapon.BP_BaseWeapon_C|GetGunMesh _asbp_base_weapon) true :!class /Script/Engine.PrimitiveComponent))
    (:then_1
      (bind _asbp_base_weapon_2 (Utilities|Casting|CastToBP_BaseWeapon (Variables|/Script/Engine.ChildActorComponent|GetChildActor (Variables|Default|GetOnlineWeapon))))
      (Class|PrimitiveComponent|SetOwnerNoSee (Variables|/HyperionOnline/Blueprints/Weapons/BP_BaseWeapon.BP_BaseWeapon_C|GetGunMesh _asbp_base_weapon_2) true))))

(fn EnterInterfaceMode
  (bind _returnvalue (Game|GetPlayerController 0))
  (bind _foundwidgets (Widget|GetAllWidgetsOfClass "/HyperionUI/Widgets/Chat/HyperionUI_ChatWindow.HyperionUI_ChatWindow_C" false))
  (for _array_element _foundwidgets
    (Variables|/Script/Engine.PlayerController|SetbShowMouseCursor _returnvalue true)
    (Input|SetInputModeGameandUI _returnvalue _array_element "DoNotLock" true)
    (Development|PrintString "Enter Interface Mode.")))

(fn DisableInterfaceMode
  (bind _returnvalue (Game|GetPlayerController 0))
  (Variables|/Script/Engine.PlayerController|SetbShowMouseCursor _returnvalue false)
  (Input|SetInputModeGameOnly _returnvalue)
  (Development|PrintString "Exit Interface Mode."))

(fn OnRepPlayerName
  (CallFunction|PopulateNameTag (Variables|Default|GetNameWidget)))

(fn PopulateNameTag
  (params (Widget :type Widget%20Component%20Object%20Reference))
  (if (not (Networking|IsDedicatedServer))
    (bind _returnvalue (UserInterface|CreateWidget "/HyperionUI/Widgets/Others/HyperionUI_Nametag.HyperionUI_Nametag_C"))
    (bind _output_get (Variables|Default|SetTagReference _returnvalue))
    (UserInterface|SetWidget Widget _output_get)
    (Default|SetNameText _returnvalue (Variables|Info|GetPlayerName))))

(fn SendNametoServer
  (CallFunction|UpdateNameonServer (PlayerState|GetPlayerName (Variables|Default|GetPlayerState))))

(fn DestroyDiscordConnection
  (params (Reason :type EEndPlayReason%20Enum :default "Destroyed"))
  (if (Utilities|Enum|Equal(Enum) Reason "Quit")
    (Class|HOCharacter|DisconnectfromDiscord)))